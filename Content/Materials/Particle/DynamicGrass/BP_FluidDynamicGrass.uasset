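; BP_FluidDynamicGrass is an actor that configures a Niagara dynamic grass system to work with a fluid field.
; BeginPlay passes it the render target size from MPC_FluidField, plus wind strength, strand attraction settings and a player height offset from the actor's Z.
; Tick copies the field's world center from the same parameter collection into Niagara, keeping the grass aligned as that center changes.
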(event EventBeginPlay
  (bind _returnvalue (Rendering|Material|GetScalarParameterValue "/Game/Materials/FoliageInteraction/Materials/MPC_FluidField.MPC_FluidField" "RT_Size" :!class /Script/Engine.KismetMaterialLibrary))
  (Niagara|SetNiagaraVariable(Float) (Variables|Default|GetNiagara) "RTSize" _returnvalue)
  (Niagara|SetNiagaraVariable(Float) (Variables|Default|GetNiagara) "WindStrengthMultiplier" (Variables|Default|GetWindStrength))
  (Niagara|SetNiagaraVariable(Float) (Variables|Default|GetNiagara) "PlayerHeight" (+ (.z (Transformation|GetActorLocation)) (Variables|Default|GetPlayerHeight)))
  (Niagara|SetNiagaraVariable(Float) (Variables|Default|GetNiagara) "StrandAttractionRadius" (Variables|Default|GetStrandAttractionRadius))
  (Niagara|SetNiagaraVariable(Float) (Variables|Default|GetNiagara) "StrandAttractionStrength" (Variables|Default|GetStrandAttractionStrength)))

(event Collision|EventActorBeginOverlap
  (params (OtherActor :type Actor%20Object%20Reference)))

(event EventTick
  (params (DeltaSeconds :type Float%20%28single-precision%29))
  (bind _returnvalue (Rendering|Material|GetVectorParameterValue "/Game/Materials/FoliageInteraction/Materials/MPC_FluidField.MPC_FluidField" "RT_WorldCenter" :!class /Script/Engine.KismetMaterialLibrary))
  (Class|NiagaraComponent|SetVariableVec2 (Variables|Default|GetNiagara) "RTCenter" (Math|Vector2D|MakeVector2D (.r _returnvalue) (.g _returnvalue))))

(fn ConstructionScript)