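; Manager actor for foliage interaction that maintains two player-centered render target fields, one for fluid forces and one fed by temperature.
; Each tick it scrolls both by the grid-snapped player movement, running update materials into buffer targets and copying back.
; It then draws each in-range listed actor using its BPC_FluidFieldInteractor settings, velocity and position.
; The field center is published to MPC_FluidField.
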(event EventBeginPlay
  (Utilities|FlowControl|Sequence
    (:then_0
      ;[0.15 0.15 0.15 0.5] Prepare RT canvas and material instance for drawing
      (bind _returnvalue (Rendering|Material|GetScalarParameterValue "/Game/Materials/FoliageInteraction/MPC_FluidField.MPC_FluidField" "RT_Size" :!class /Script/Engine.KismetMaterialLibrary))
      (Variables|Default|SetRT_Size _returnvalue)
      (bind _returnvalue_2 (Rendering|Material|CreateDynamicMaterialInstance "/Game/Materials/FoliageInteraction/M_FluidInjection.M_FluidInjection" "None" "None" :!class /Script/Engine.KismetMaterialLibrary))
      (Variables|Default|SetFluidInjectionDynamic _returnvalue_2)
      (bind _returnvalue_3 (Rendering|Material|CreateDynamicMaterialInstance "/Game/Materials/FoliageInteraction/M_Update.M_Update" "None" "None" :!class /Script/Engine.KismetMaterialLibrary))
      (Variables|Default|SetUpdateDynamic _returnvalue_3)
      (bind _returnvalue_4 (Rendering|Material|CreateDynamicMaterialInstance "/Game/Materials/FoliageInteraction/M_Copy.M_Copy" "None" "None" :!class /Script/Engine.KismetMaterialLibrary))
      (Variables|Default|SetCopyDynamic _returnvalue_4)
      (Variables|Default|SetLastCenterLocation (Class|KismetMathLibrary|VectorSnappedtoGrid (Transformation|GetActorLocation (Game|Player|GetPlayerPawn 0)) (Variables|Default|GetSnapGridSize)))
      (Rendering|ClearRenderTarget2D "/Game/Materials/FoliageInteraction/RT_FluidField.RT_FluidField" "(R=0.000000,G=0.000000,B=0.000000,A=0.000000)")
      (Rendering|ClearRenderTarget2D "/Game/Materials/FoliageInteraction/RT_Buffer.RT_Buffer" "(R=0.000000,G=0.000000,B=0.000000,A=0.000000)"))
    (:then_1
      ;[0.15 0.15 0.15 0.5] Prepare RT canvas and material instance for drawing
      (bind _returnvalue_5 (Rendering|Material|GetScalarParameterValue "/Game/Materials/FoliageInteraction/MPC_FluidField.MPC_FluidField" "RT_Size" :!class /Script/Engine.KismetMaterialLibrary))
      (Variables|Default|SetRT_Size _returnvalue_5)
      (bind _returnvalue_6 (Rendering|Material|CreateDynamicMaterialInstance "/Game/Materials/FoliageInteraction/M_FluidInjection_1.M_FluidInjection_1" "None" "None" :!class /Script/Engine.KismetMaterialLibrary))
      (Variables|Default|SetFluidInjectionDynamic_1 _returnvalue_6)
      (bind _returnvalue_7 (Rendering|Material|CreateDynamicMaterialInstance "/Game/Materials/FoliageInteraction/M_Update_1.M_Update_1" "None" "None" :!class /Script/Engine.KismetMaterialLibrary))
      (Variables|Default|SetUpdateDynamic_1 _returnvalue_7)
      (bind _returnvalue_8 (Rendering|Material|CreateDynamicMaterialInstance "/Game/Materials/FoliageInteraction/M_Copy.M_Copy" "None" "None" :!class /Script/Engine.KismetMaterialLibrary))
      (Variables|Default|SetCopyDynamic_1 _returnvalue_8)
      (Variables|Default|SetLastCenterLocation (Class|KismetMathLibrary|VectorSnappedtoGrid (Transformation|GetActorLocation (Game|Player|GetPlayerPawn 0)) (Variables|Default|GetSnapGridSize)))
      (Rendering|ClearRenderTarget2D "/Game/Materials/FoliageInteraction/RT_FluidField_1.RT_FluidField_1" "(R=0.000000,G=0.000000,B=0.000000,A=0.000000)")
      (Rendering|ClearRenderTarget2D "/Game/Materials/FoliageInteraction/RT_Buffer_1.RT_Buffer_1" "(R=0.000000,G=0.000000,B=0.000000,A=0.000000)"))))

(event Collision|EventActorBeginOverlap
  (params (OtherActor :type Actor%20Object%20Reference)))

(event EventTick
  (params (DeltaSeconds :type Float%20%28single-precision%29))
  (bind _updatedynamic (Variables|Default|GetUpdateDynamic))
  (bind _copydynamic (Variables|Default|GetCopyDynamic))
  (bind _updatedynamic_1 (Variables|Default|GetUpdateDynamic_1))
  (bind _copydynamic_1 (Variables|Default|GetCopyDynamic_1))
  (bind _rt_size (Variables|Default|GetRT_Size))
  ;[0.15 0.15 0.15 0.5] Calculated movement compensation from last frame
  (bind _output_get (Variables|Default|SetCurrentCenterLocation (Class|KismetMathLibrary|VectorSnappedtoGrid (Transformation|GetActorLocation (Game|Player|GetPlayerPawn 0)) (Variables|Default|GetSnapGridSize))))
  (Variables|Default|SetDeltaUV (Math|Vector|MakeVector (/ (.x (- _output_get (Variables|Default|GetLastCenterLocation))) _rt_size) (/ (.y (- _output_get (Variables|Default|GetLastCenterLocation))) _rt_size) 0.0))
  ;[0.15 0.15 0.15 0.5] Use buffer RT to store temperary update result from last frame then write back to main render target
  (Rendering|Material|SetTextureParameterValue _updatedynamic "PreviousRT" "/Game/Materials/FoliageInteraction/RT_FluidField.RT_FluidField")
  (Rendering|Material|SetVectorParameterValue _updatedynamic "DeltaUV" (Math|Conversions|ToLinearColor(Vector) (Variables|Default|GetDeltaUV)) :!class /Script/Engine.MaterialInstanceDynamic)
  (Rendering|ClearRenderTarget2D "/Game/Materials/FoliageInteraction/RT_Buffer.RT_Buffer" "(R=0.000000,G=0.000000,B=0.000000,A=0.000000)")
  (Rendering|DrawMaterialtoRenderTarget "/Game/Materials/FoliageInteraction/RT_Buffer.RT_Buffer" _updatedynamic)
  (Rendering|Material|SetTextureParameterValue _copydynamic "BufferRT" "/Game/Materials/FoliageInteraction/RT_Buffer.RT_Buffer")
  (Rendering|ClearRenderTarget2D "/Game/Materials/FoliageInteraction/RT_FluidField.RT_FluidField" "(R=0.000000,G=0.000000,B=0.000000,A=0.000000)")
  (Rendering|DrawMaterialtoRenderTarget "/Game/Materials/FoliageInteraction/RT_FluidField.RT_FluidField" _copydynamic)
  ;[0.15 0.15 0.15 0.5] Use buffer RT to store temperary update result from last frame then write back to main render target
  (Rendering|Material|SetTextureParameterValue _updatedynamic_1 "PreviousRT" "/Game/Materials/FoliageInteraction/RT_FluidField_1.RT_FluidField_1")
  (Rendering|Material|SetVectorParameterValue _updatedynamic_1 "DeltaUV" (Math|Conversions|ToLinearColor(Vector) (Variables|Default|GetDeltaUV)) :!class /Script/Engine.MaterialInstanceDynamic)
  (Rendering|ClearRenderTarget2D "/Game/Materials/FoliageInteraction/RT_Buffer_1.RT_Buffer_1" "(R=0.000000,G=0.000000,B=0.000000,A=0.000000)")
  (Rendering|DrawMaterialtoRenderTarget "/Game/Materials/FoliageInteraction/RT_Buffer_1.RT_Buffer_1" _updatedynamic_1)
  (Rendering|Material|SetTextureParameterValue _copydynamic_1 "BufferRT" "/Game/Materials/FoliageInteraction/RT_Buffer_1.RT_Buffer_1")
  (Rendering|ClearRenderTarget2D "/Game/Materials/FoliageInteraction/RT_FluidField_1.RT_FluidField_1" "(R=0.000000,G=0.000000,B=0.000000,A=0.000000)")
  (Rendering|DrawMaterialtoRenderTarget "/Game/Materials/FoliageInteraction/RT_FluidField_1.RT_FluidField_1" _copydynamic_1)
  ;[0.15 0.15 0.15 0.5] Iterate all actors for rendering (TODO: move the logic to c++)
  (bind _valuepin (Utilities|Set|ForEachLoop(Set) (Variables|Default|GetActorList))
    (:then
      (CallFunction|DrawRenderTarget _valuepin))
    (:CompletedPin
      ;[0.15 0.15 0.15 0.5] Update last center
      (bind _output_get_2 (Variables|Default|SetLastCenterLocation (Variables|Default|GetCurrentCenterLocation)))
      (Rendering|Material|SetVectorParameterValue "/Game/Materials/FoliageInteraction/MPC_FluidField.MPC_FluidField" "RT_WorldCenter" (Math|Conversions|ToLinearColor(Vector) (Class|KismetMathLibrary|VectorSnappedtoGrid _output_get_2 (Variables|Default|GetSnapGridSize))) :!class /Script/Engine.KismetMaterialLibrary))))

(fn ConstructionScript)

(fn DrawRenderTarget
  (params (InputPin :type Actor%20Object%20Reference))
  (bind _returnvalue (Transformation|GetActorLocation InputPin))
  (LocalVariables|SetFFComponent (Actor|GetComponentbyClass InputPin "/Game/Materials/FoliageInteraction/BPC_FluidFieldInteractor.BPC_FluidFieldInteractor_C"))
  (if (<= (Math|Vector|VectorLength (- (Variables|Default|GetCurrentCenterLocation) _returnvalue)) (/ (Variables|Default|GetRT_Size) 2.0))
    ;[0.15 0.15 0.15 0.5] Set injection material parameters
    (Rendering|Material|SetVectorParameterValue (Variables|Default|GetFluidInjectionDynamic_1) "ActorCenter" (Math|Conversions|ToLinearColor(Vector) (+ (/ (- _returnvalue (Variables|Default|GetCurrentCenterLocation)) (Variables|Default|GetRT_Size)) 0.5)) :!class /Script/Engine.MaterialInstanceDynamic)
    (Rendering|Material|SetScalarParameterValue (Variables|Default|GetFluidInjectionDynamic) "ActorDynamicRadius" (Variables|/Game/Materials/FoliageInteraction/BPC_FluidFieldInteractor.BPC_FluidFieldInteractor_C|GetStaticRadius (LocalVariables|GetFFComponent)) :!class /Script/Engine.MaterialInstanceDynamic)
    (Rendering|Material|SetScalarParameterValue (Variables|Default|GetFluidInjectionDynamic_1) "ActorStaticRadius" (Variables|/Game/Materials/FoliageInteraction/BPC_FluidFieldInteractor.BPC_FluidFieldInteractor_C|GetStaticRadius (LocalVariables|GetFFComponent)) :!class /Script/Engine.MaterialInstanceDynamic)
    (Rendering|Material|SetVectorParameterValue (Variables|Default|GetFluidInjectionDynamic) "ActorVelocity" (Math|Conversions|ToLinearColor(Vector) (* (Transformation|GetVelocity InputPin) (Variables|/Game/Materials/FoliageInteraction/BPC_FluidFieldInteractor.BPC_FluidFieldInteractor_C|GetDynamicVelocityScale (LocalVariables|GetFFComponent)))) :!class /Script/Engine.MaterialInstanceDynamic)
    (Rendering|Material|SetScalarParameterValue (Variables|Default|GetFluidInjectionDynamic) "StaticForceMultiplier" (Variables|/Game/Materials/FoliageInteraction/BPC_FluidFieldInteractor.BPC_FluidFieldInteractor_C|GetStaticForceMultiplier (LocalVariables|GetFFComponent)) :!class /Script/Engine.MaterialInstanceDynamic)
    (Rendering|Material|SetScalarParameterValue (Variables|Default|GetFluidInjectionDynamic) "ActorWorldZ" (/ (.z (Transformation|GetActorLocation InputPin)) 1e+02) :!class /Script/Engine.MaterialInstanceDynamic)
    (Rendering|Material|SetScalarParameterValue (Variables|Default|GetFluidInjectionDynamic_1) "InputTemperature" (Variables|/Game/Materials/FoliageInteraction/BPC_FluidFieldInteractor.BPC_FluidFieldInteractor_C|GetTemperature (LocalVariables|GetFFComponent)) :!class /Script/Engine.MaterialInstanceDynamic)
    ;[0.15 0.15 0.15 0.5] Draw render target
    (Rendering|DrawMaterialtoRenderTarget "/Game/Materials/FoliageInteraction/RT_FluidField.RT_FluidField" (Variables|Default|GetFluidInjectionDynamic))
    (Rendering|DrawMaterialtoRenderTarget "/Game/Materials/FoliageInteraction/RT_FluidField_1.RT_FluidField_1" (Variables|Default|GetFluidInjectionDynamic_1))))